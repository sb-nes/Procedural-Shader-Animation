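; BP_RandomPointInShape is an actor that spawns a given actor class at a random point inside its Box component.
; The Spawn event picks the point around the root's world location using the box's unscaled extent, so box rotation and scale are ignored.
; It then sets the spawned root's world rotation to either a random pitch and roll with zero yaw, or zero rotation, according to the RandomRotation flag.
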(event `self.ReceiveBeginPlay`)

(event `Spawn`
  (params (Actor :type "Actor Class Reference") (`Random Rotation` :type Boolean))
  (set `self.Random Rotation` `Random Rotation`)
  (bind _returnvalue (`|SpawnActorFromClass` Actor (`KismetMathLibrary.MakeTransform` (`KismetMathLibrary.RandomPointInBoundingBox` (`SceneComponent.K2_GetComponentLocation` (`self.DefaultSceneRoot`)) (`BoxComponent.BoxExtent` (`self.Box`)))) "Undefined" "OverrideRootScale" null null))
  (`SceneComponent.K2_SetWorldRotation` (`Actor.RootComponent` _returnvalue) (`KismetMathLibrary.SelectRotator` (`KismetMathLibrary.MakeRotator` (`KismetMathLibrary.RandomFloatInRange` -90.0 90.0) (`KismetMathLibrary.RandomFloatInRange` -90.0 90.0)) (struct) (`self.Random Rotation`)) false false))

(fn `UserConstructionScript`)