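; BP_TimedSpawner is a spawner actor that periodically produces red blood cells (BP_Erythrocytes) and neutrophil NPCs.
; On BeginPlay it starts two looping timers, with red blood cells on the faster one, and caches the player's BL_Pawn.
; Each timer calls Spawn for its cell type without random rotation.
; The red blood cell timer also adds one to the first InformationArray entry on the pawn's main HUD.
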(event `self.ReceiveBeginPlay`
  (`parent.ReceiveBeginPlay`)
  (`KismetSystemLibrary.K2_SetTimer` null "TimerRBC" 1.0 true)
  (bind _asbl_pawn (cast `/Game/GameBP/BL_Pawn` (`GameplayStatics.GetPlayerPawn` 0)))
  (set `self.PawnRef` _asbl_pawn)
  (`KismetSystemLibrary.K2_SetTimer` null "TimerNeutrophils" 3.5 true))

(event `TimerRBC`
  (bind _pawnref (`self.PawnRef`))
  (`self.Spawn` "/Game/Blueprints/Actors/Cells/BP_Erythrocytes.BP_Erythrocytes_C")
  (`/Engine/EditorBlueprintResources/StandardMacros.IsValid` _pawnref
    (:`Is Valid`
      (`/Game/UMG/W_Information.Add` (`|GetArrayItem` (`/Game/UMG/W_MainHUD.InformationArray` (`/Game/GameBP/BL_Pawn.MainHUDRef` _pawnref))) 1))))

(event `TimerNeutrophils`
  (`self.Spawn` "/Game/Blueprints/AI/NPC/NPC_Neutrophil.NPC_Neutrophil_C"))

(fn `UserConstructionScript`
  (`parent.UserConstructionScript`))